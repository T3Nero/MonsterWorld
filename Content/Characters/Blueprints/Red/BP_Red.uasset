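; BP_Red is the player-controlled Paper2D top-down character Red, with movement, interaction, a HUD and a quit input.
; On BeginPlay it creates the HUD and adds the top-down Enhanced Input mapping context.
; Move input drives movement and stores the last direction, which selects four-way walk or idle flipbooks, favoring horizontal.
; Interact messages the first overlapping BPI_Interact actor, passing the HUD, then hides the message box after a retriggerable delay.
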(event Input|EnhancedActionEvents|EnhancedInputActionIA_Move
  (params (ActionValue :type Vector%202D%20Structure) (ElapsedSeconds :type Float%20%28double-precision%29) (TriggeredSeconds :type Float%20%28double-precision%29) (InputAction :type Input%20Action%20Object%20Reference :default "/Game/Input/Actions/IA_Move.IA_Move"))
  (bind (_x _y) (Math|Vector2D|BreakVector2D ActionValue))
  ;[1 1 1] IA_Move : Handle Sprite Movement Input
  (:Triggered
    (Variables|Default|SetLastDirection ActionValue)
    (Pawn|Input|AddMovementInput "1.000000,0.000000,0.000000" _x false)
    (Pawn|Input|AddMovementInput "0.000000,1.000000,0.000000" _y false)
    (CallFunction|UpdateAnimations false))
  (:Completed
    (CallFunction|UpdateAnimations true)))

(event Input|EnhancedActionEvents|EnhancedInputActionIA_Exit
  (params (ActionValue :type Boolean) (ElapsedSeconds :type Float%20%28double-precision%29) (TriggeredSeconds :type Float%20%28double-precision%29) (InputAction :type Input%20Action%20Object%20Reference :default "/Game/Input/Actions/IA_Exit.IA_Exit"))
  (:Started
    (Game|QuitGame 0 "Quit" false)))

(event Input|EnhancedActionEvents|EnhancedInputActionIA_Interact
  (params (ActionValue :type Boolean) (ElapsedSeconds :type Float%20%28double-precision%29) (TriggeredSeconds :type Float%20%28double-precision%29) (InputAction :type Input%20Action%20Object%20Reference :default "/Game/Input/Actions/IA_Interact.IA_Interact"))
  (:Started
    (bind _array_element (Utilities|Array|ForEachLoopwithBreak (Collision|GetOverlappingActors (Variables|Default|GetInteractBox) 0 :!class /Script/Engine.PrimitiveComponent) :!label _label)
      (:LoopBody
        (if (Utilities|DoesObjectImplementInterface _array_element "/Game/Characters/Blueprints/BPI_Interact.BPI_Interact_C")
          (Class|BPIInteract|Interact(Message) _array_element (Variables|Default|GetWBPHUD))
          (goto _label Break)))
      (:Completed
        (Utilities|FlowControl|RetriggerableDelay (Variables|Default|GetHideMessageDelay))
        (Widget|SetVisibility (Variables|/Game/UI/WBP_HUD.WBP_HUD_C|GetWBP_MessageBox (Variables|Default|GetWBPHUD)) "Hidden")))))

(event EventBeginPlay
  (bind _returnvalue (UserInterface|CreateWidget "/Game/UI/WBP_HUD.WBP_HUD_C"))
  (bind _output_get (Variables|Default|SetWBPHUD _returnvalue))
  (UserInterface|Viewport|AddtoViewport _output_get 0)
  (Class|WidgetBlueprintLibrary|SetFocustoGameViewport)
  (Input|AddMappingContext (PlayerController|LocalPlayerSubsystems|GetEnhancedInputLocalPlayerSubsystem (Game|GetPlayerController 0)) "/Game/Input/IMC_TopDown.IMC_TopDown" 0 "(bIgnoreAllPressedKeysUntilRelease=True,bForceImmediately=False,bNotifyUserSettings=False)"))

(fn ConstructionScript)

(fn UpdateAnimations
  (params (TransitionToIdle :type Boolean))
  (if TransitionToIdle
    (Math|Float|CompareFloat (.X (Math|Vector2D|BreakVector2D (Variables|Default|GetLastDirection))) 0.0
      (:>
        (Sprite|SetFlipbook (Variables|Default|GetSprite) "/Game/PaperAssets/Characters/Red/Flipbooks/FB_Red_Idle_R.FB_Red_Idle_R"))
      (:==
        (Math|Float|CompareFloat (.Y (Math|Vector2D|BreakVector2D (Variables|Default|GetLastDirection))) 0.0
          (:>
            (Sprite|SetFlipbook (Variables|Default|GetSprite) "/Game/PaperAssets/Characters/Red/Flipbooks/FB_Red_Idle_D.FB_Red_Idle_D"))
          (:<
            (Sprite|SetFlipbook (Variables|Default|GetSprite) "/Game/PaperAssets/Characters/Red/Flipbooks/FB_Red_Idle_U.FB_Red_Idle_U"))))
      (:<
        (Sprite|SetFlipbook (Variables|Default|GetSprite) "/Game/PaperAssets/Characters/Red/Flipbooks/FB_Red_Idle_L.FB_Red_Idle_L")))
    (else
      (Math|Float|CompareFloat (.X (Math|Vector2D|BreakVector2D (Variables|Default|GetLastDirection))) 0.0
        (:>
          (Sprite|SetFlipbook (Variables|Default|GetSprite) "/Game/PaperAssets/Characters/Red/Flipbooks/FB_Red_Walk_R.FB_Red_Walk_R"))
        (:==
          (Math|Float|CompareFloat (.Y (Math|Vector2D|BreakVector2D (Variables|Default|GetLastDirection))) 0.0
            (:>
              (Sprite|SetFlipbook (Variables|Default|GetSprite) "/Game/PaperAssets/Characters/Red/Flipbooks/FB_Red_Walk_D.FB_Red_Walk_D"))
            (:<
              (Sprite|SetFlipbook (Variables|Default|GetSprite) "/Game/PaperAssets/Characters/Red/Flipbooks/FB_Red_Walk_U.FB_Red_Walk_U"))))
        (:<
          (Sprite|SetFlipbook (Variables|Default|GetSprite) "/Game/PaperAssets/Characters/Red/Flipbooks/FB_Red_Walk_L.FB_Red_Walk_L"))))))